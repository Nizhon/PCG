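; Master spline Blueprint that builds vertically layered meshes along a spline in its construction script.
; Bottom mesh X extent times ScaleSplit sets segment length, rounded to divide the spline evenly and shared by all layers.
; Bottom, repeated middle and top layers stack by accumulated Z offsets, with middle and top optional.
; Each segment becomes a spline mesh component with tangents clamped to segment length, the last ending on a spline point.
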(fn `Get Length and Spacing`
  (params (BaseMesh :type "StaticMesh Object Reference"))
  (returns (MeshDivisions :type Integer))
  (bind _returnvalue (`SplineComponent.GetSplineLength` (`self.Spline`)))
  (bind _returnvalue_2 (`KismetMathLibrary.Round` (/ _returnvalue (`self.Mesh_Length`))))
  (set `self.Mesh_Length` (* (.x (`.BoxExtent` (`KismetMathLibrary.BreakBoxSphereBounds` (`StaticMesh.GetBounds` BaseMesh)))) (`self.Scale_Split`)))
  (set `self.Spline_Spacing` (/ _returnvalue (`KismetMathLibrary.Conv_IntToDouble` _returnvalue_2)))
  (return (- _returnvalue_2 1)))

(fn `SetMeshSpline`
  (params (`Spline Divisions` :type Integer) (`Relative Transform` :type "Transform Structure") (Mesh :type "StaticMesh Object Reference"))
  (bind _spline (`self.Spline`))
  (bind _spline_2 (`self.Spline`))
  (bind _spline_3 (`self.Spline`))
  (for _index (range (+ `Spline Divisions` 1))
    (bind _returnvalue (`AddComponent|NODE_AddSplineMeshComponent-2` :`RelativeTransform` `Relative Transform`))
    (`StaticMeshComponent.SetStaticMesh` _returnvalue Mesh)
    (if (!= `Spline Divisions` _index)
      (bind _returnvalue_2 (* _index (`self.Spline_Spacing`)))
      (bind _returnvalue_3 (`SplineComponent.GetLocationAtDistanceAlongSpline` _spline_3 _returnvalue_2 "Local"))
      (bind _returnvalue_4 (`KismetMathLibrary.ClampVectorSize` (`SplineComponent.GetTangentAtDistanceAlongSpline` _spline_3 _returnvalue_2 "Local") 0.0 (`self.Mesh_Length`)))
      (bind _returnvalue_5 (* (+ _index 1) (`self.Spline_Spacing`)))
      (`SplineMeshComponent.SetStartAndEnd` _returnvalue _returnvalue_3 _returnvalue_4 (`SplineComponent.GetLocationAtDistanceAlongSpline` _spline_2 _returnvalue_5 "Local") (`KismetMathLibrary.ClampVectorSize` (`SplineComponent.GetTangentAtDistanceAlongSpline` _spline_2 _returnvalue_5 "Local") 0.0 (`self.Mesh_Length`)) true)
      (else
        (bind _returnvalue_6 (+ _index 1))
        (`SplineMeshComponent.SetStartAndEnd` _returnvalue _returnvalue_3 _returnvalue_4 (`SplineComponent.GetLocationAtSplinePoint` _spline _returnvalue_6 "Local") (`KismetMathLibrary.ClampVectorSize` (`SplineComponent.GetTangentAtSplinePoint` _spline _returnvalue_6 "Local") 0.0 (`self.Mesh_Length`)) true)))))

(fn `UserConstructionScript`
  (bind _meshdivisions (`self.Get Length and Spacing` (`self.Bottom_Mesh`)))
  (`self.SetMeshSpline` _meshdivisions (struct) (`self.Bottom_Mesh`))
  (for _ (range 1 (+ (`self.Vertical Tile Amount`) 1))
    (set `self.Total Offset` (+ (`KismetMathLibrary.MakeVector` 0.0 0.0 (`self.Vertical Offset Mid`)) (`self.Total Offset`)))
    (`/Engine/EditorBlueprintResources/StandardMacros.IsValid` (`self.Mid_Mesh`)
      (:`Is Valid`
        (`self.SetMeshSpline` _meshdivisions (`KismetMathLibrary.MakeTransform` (`self.Total Offset`)) (`self.Mid_Mesh`)))))
  (set `self.Total Offset` (+ (`KismetMathLibrary.MakeVector` 0.0 0.0 (`self.Vertical Offset Top`)) (`self.Total Offset`)))
  (`/Engine/EditorBlueprintResources/StandardMacros.IsValid` (`self.Top_Mesh`)
    (:`Is Valid`
      (`self.SetMeshSpline` _meshdivisions (`KismetMathLibrary.MakeTransform` (`self.Total Offset`)) (`self.Top_Mesh`)))))