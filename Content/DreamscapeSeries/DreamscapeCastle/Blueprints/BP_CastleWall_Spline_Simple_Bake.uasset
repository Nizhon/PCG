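; Castle wall spline tool that lines a spline with randomly picked wall meshes and can bake them into standalone actors.
; The construction script derives spacing from a random mesh's X bounds plus an offset, then adds mesh components along the spline.
; Each piece is aimed at the next spline point, with its rotation scaled by a multiplier.
; BakeOutMeshes replaces each generated component with a StaticMeshActor at the same world transform.
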(event `Bake Out Meshes`
  (for _array_element (`self.AllCreatedStaticMeshes`)
    (bind _returnvalue (`|SpawnActorFromClass` "/Script/Engine.StaticMeshActor" (`SceneComponent.K2_GetComponentToWorld` _array_element) "Undefined" "OverrideRootScale" null null))
    (`StaticMeshComponent.SetStaticMesh` (`StaticMeshActor.StaticMeshComponent` _returnvalue) (`StaticMeshComponent.StaticMesh` _array_element))
    (`ActorComponent.K2_DestroyComponent` _array_element)))

(fn `GetLocationAtIndex`
  (params (A :type Integer))
  (returns (ReturnValue :type "Vector Structure"))
  (return (`SplineComponent.GetLocationAtDistanceAlongSpline` (`self.Spline`) (* A (`self.MeshSpacing`)) "Local")))

(fn `UserConstructionScript`
  (bind _outitem (`KismetArrayLibrary.Array_Random` (`self.PlacedMesh`)))
  (bind (_min _max) (break `Box` (`StaticMesh.GetBoundingBox` _outitem)))
  (bind _output_get (set `self.MeshSpacing` (+ (.x (- _max _min)) (`self.MeshOffset`))))
  (bind _output_get_2 (set `self.NumberOfInstances` (`KismetMathLibrary.FFloor` (/ (`SplineComponent.GetSplineLength` (`self.Spline`)) _output_get))))
  (for _index (range (+ _output_get_2 1))
    (bind _returnvalue (`self.GetLocationAtIndex` _index))
    (bind _returnvalue_2 (`self.GetLocationAtIndex` (+ _index 1)))
    (bind _returnvalue_3 (`AddComponent|NODE_AddStaticMeshComponent-1` :`RelativeTransform` (`KismetMathLibrary.MakeTransform` _returnvalue (* (`KismetMathLibrary.MakeRotFromX` (- _returnvalue_2 _returnvalue)) (`self.MeshRotationMultiplier`)))))
    (bind _output_get_3 (set `self.CreatedStaticMesh` _returnvalue_3))
    (`KismetArrayLibrary.Array_Add` (`self.AllCreatedStaticMeshes`) _output_get_3)
    (`StaticMeshComponent.SetStaticMesh` _returnvalue_3 _outitem)))