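; BP_Building is a procedural building actor that drives a PCG graph from its wall size, floor size and floor count.
; The construction script converts these into graph parameters for floor scale, wall, beam and roof offsets, building height and a single-floor flag.
; It also passes the negated actor location as the floor copy offset.
; Roof height uses a fixed per-floor step rather than WallSize, and the event graph is empty.
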(event EventBeginPlay)

(event Collision|EventActorBeginOverlap
  (params (OtherActor :type Actor%20Object%20Reference)))

(event EventTick
  (params (DeltaSeconds :type Float%20%28single-precision%29)))

(fn ConstructionScript
  (bind _pcg (Variables|Default|GetPCG))
  (bind _wallsize (Variables|Default|GetWallSize))
  (bind _floors (Variables|Default|GetFloors))
  (bind _returnvalue (* _wallsize -0.5))
  (bind _graphinstance (Variables|/Script/PCG.PCGComponent|GetGraphInstance _pcg))
  (bind _returnvalue_2 (* _returnvalue -1.0))
  (Effects|Components|ParticleSystem|SetVectorParameter _graphinstance "FloorScale" (Math|Conversions|ToVector(Float) (/ (Variables|Default|GetWallSize) (Variables|Default|GetFloorSize))))
  (Effects|Components|ParticleSystem|SetVectorParameter _graphinstance "WallOffset1" (Math|Vector|MakeVector _returnvalue 0.0 0.0))
  (Effects|Components|ParticleSystem|SetVectorParameter _graphinstance "WallOffset2" (Math|Vector|MakeVector _returnvalue_2 0.0 0.0))
  (Effects|Components|ParticleSystem|SetVectorParameter _graphinstance "WallOffset3" (Math|Vector|MakeVector 0.0 _returnvalue 0.0))
  (Effects|Components|ParticleSystem|SetVectorParameter _graphinstance "WallOffset4" (Math|Vector|MakeVector 0.0 _returnvalue_2 0.0))
  (Effects|Components|ParticleSystem|SetVectorParameter _graphinstance "BuildingHeight" (Math|Vector|MakeVector 0.0 0.0 (* (Variables|Default|GetWallSize) (- (Variables|Default|GetFloors) 1))))
  (Effects|Components|ParticleSystem|SetVectorParameter _graphinstance "FloorCopyOffset" (* (Transformation|GetActorLocation) -1.0))
  (Effects|Components|ParticleSystem|SetBoolParameter _graphinstance "SingleFloor" (== _floors 1))
  (Effects|Components|ParticleSystem|SetVectorParameter _graphinstance "RoofOffset" (Math|Vector|MakeVector 0.0 0.0 (Math|Conversions|ToFloat(Integer) (* _floors 400))))
  (Effects|Components|ParticleSystem|SetVectorParameter _graphinstance "RoofPivotOffset" (Math|Vector|MakeVector 0.0 (/ (Variables|Default|GetWallSize) 2.0) 0.0))
  (Effects|Components|ParticleSystem|SetVectorParameter _graphinstance "BeamOffset" (Math|Vector|MakeVector (/ (Variables|Default|GetWallSize) 2.0) 0.0 0.0)))