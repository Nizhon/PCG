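; Custom PCG node for house generation, titled "Select Random Points", that marks a random subset of input points by overriding their density.
; For each spatial input, it converts to point data, shuffles point indices and takes up to PointAmount of them.
; Selected points get DensityToSet, and all points are output with original tags and pins.
; Shuffling ignores the PCG seed, and index arrays are not cleared between inputs.
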(fn ExecutewithContext
  (params (InContext :type PCG%20Context%20Structure%20%28by%20ref%29) (Input :type PCG%20Data%20Collection%20Structure%20%28by%20ref%29))
  (bind _returnvalue (Class|PCGDataFunctionLibrary|GetInputs Input))
  (for _array_element _returnvalue
    (bind _aspcgspatial_data (Utilities|Casting|CastToPCGSpatialData (.Data (Utilities|Struct|BreakPCGTaggedData _array_element))))
    (bind _output_get (LocalVariables|SetPCGPointData (SpatialData|ToPointDatawithContext _aspcgspatial_data InContext)))
    (bind _output_get_2 (LocalVariables|SetPCGPoints (SpatialData|GetPoints _output_get)))
    (LocalVariables|SetPointCount (Utilities|Array|Length _output_get_2))
    (LocalVariables|SetSelectedMaxPoints (> (Variables|Default|GetPointAmount) (LocalVariables|GetPointCount)))
    (for _index (range 0 (LocalVariables|GetPointCount))
      (Utilities|Array|Add (LocalVariables|GetIndexTracker) _index))
    (Utilities|Array|Shuffle (LocalVariables|GetIndexTracker))
    (if (LocalVariables|GetSelectedMaxPoints)
      (Variables|Default|SetPointAmount (+ (LocalVariables|GetPointCount) 1)))
    (for _index_2 (range 1 (Variables|Default|GetPointAmount))
      (Utilities|Array|Add (LocalVariables|GetIndexesToSelect) (Utilities|Array|Get(acopy) (LocalVariables|GetIndexTracker) _index_2)))
    (for (_array_element_2 _array_index) (LocalVariables|GetPCGPoints)
      (for _array_element_3 (LocalVariables|GetIndexesToSelect)
        (if (== _array_element_3 _array_index)
          (bind _structout (Utilities|Struct|SetmembersinPCGPoint _array_element_2 (Variables|Default|GetDensityToSet)))
          (Utilities|Array|SetArrayElem (LocalVariables|GetPCGPoints) _array_index _structout))))
    (SpatialData|SetPoints (LocalVariables|GetPCGPointData) (LocalVariables|GetPCGPoints))
    (Utilities|Array|Add (LocalVariables|GetOutTaggedData) (Utilities|Struct|MakePCGTaggedData (LocalVariables|GetPCGPointData) (.Tags (Utilities|Struct|BreakPCGTaggedData _array_element)) (.Pin (Utilities|Struct|BreakPCGTaggedData _array_element)))))
  (return (Utilities|Struct|MakePCGDataCollection (LocalVariables|GetOutTaggedData))))

(fn NodeTitleOverride
  (return "Select Random Points"))